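; Base AI NPC character that spots the first-person player and performs a melee attack.
; Pawn sensing sets the hasSeenPlayer blackboard key on sighting the player.
; Attack sphere-traces ahead, plays a montage, applies delayed damage without rechecking the hit, and plays its sound only once via an unreset DoOnce.
; Helper functions provide random nearby destinations and a forward line-trace obstacle check with a random sideways turn point.
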(event `self.PawnSensing.OnSeePawn`
  (params (Pawn :type "Pawn Object Reference"))
  ;[1 1 1] Ve al Player
  (cast `/Game/FirstPerson/Blueprints/BP_FirstPersonCharacter` Pawn)
  (`BlackboardComponent.SetValueAsBool` (`AIBlueprintHelperLibrary.GetBlackboard` (`AIBlueprintHelperLibrary.GetAIController` self)) "hasSeenPlayer" true))

(event `Attack`
  (bind _returnvalue (`self.K2_GetActorLocation`))
  ;[1 1 1] Attack Player
  (bind (_outhit _returnvalue_2) (`KismetSystemLibrary.SphereTraceSingleForObjects` _returnvalue (+ _returnvalue (* (`KismetMathLibrary.GetForwardVector` (`self.K2_GetActorRotation`)) 100.0)) 120.0 (`|MakeArray` "ObjectTypeQuery3" :!type "EObjectTypeQuery Enum")))
  (if _returnvalue_2
    (bind (_bblockinghit _binitialoverlap _time _distance _location _impactpoint _normal _impactnormal _physmat _hitactor) (`GameplayStatics.BreakHitResult` _outhit))
    (cast `/Game/FirstPerson/Blueprints/BP_FirstPersonCharacter` _hitactor)
    (`self.PlayAnimMontage` "/Game/NPC/NPC/AM_Attack.AM_Attack")
    (`|ExecutionSequence`
      (:`then_0`
        (`KismetSystemLibrary.Delay` 1.03)
        (`GameplayStatics.ApplyDamage` _hitactor (`self.Damage`)))
      (:`then_1`
        (`/Engine/EditorBlueprintResources/StandardMacros.DoOnce` false
          (:`Completed`
            (`GameplayStatics.PlaySound2D` "/Game/Audio/Enemy/Attack_Cue.Attack_Cue" 1.0 1.0 0.0 null null)))))))

(fn `AvoidLine`
  (returns (FrontDestination :type "Vector Structure") (HitSomething :type Boolean) (Turn :type "Vector Structure"))
  (bind _returnvalue (`self.K2_GetActorLocation`))
  (bind _returnvalue_2 (+ _returnvalue (* (`self.GetActorForwardVector`) 650)))
  (bind (_outhits _returnvalue_3) (`KismetSystemLibrary.LineTraceMulti` :`Start` _returnvalue :`End` _returnvalue_2 :`TraceChannel` "TraceTypeQuery1" :`DrawDebugType` "ForDuration"))
  (return _returnvalue_2 _returnvalue_3 (+ _returnvalue (* (`self.GetActorRightVector`) (`KismetMathLibrary.RandomIntegerInRange` -500 500)))))

(fn `Get Random Destination`
  (returns (ReturnValue :type "Vector Structure"))
  (return (+ (`self.K2_GetActorLocation` (`Controller.K2_GetPawn` (`AIBlueprintHelperLibrary.GetAIController` self))) (`KismetMathLibrary.MakeVector` (`KismetMathLibrary.RandomFloatInRange` -500.0 500.0) (`KismetMathLibrary.RandomFloatInRange` -500.0 500.0)))))

(fn `UserConstructionScript`)