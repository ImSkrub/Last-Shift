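; Key pickup actor that the player collects by walking into its collider.
; On BeginPlay it caches the first-person character, retrying the cast after a short delay until it succeeds.
; Player overlap hides and destroys the actor, adds its Key1 value to the character's Key2 and prints the total.
; The construction script applies a configurable mesh and material, and a logging custom event is never called here.
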(event `PickUp`
  (bind _mesh_base (`self.Mesh Base`))
  ;[1 1 1] PickUp
  (`PrimitiveComponent.SetCollisionEnabled` _mesh_base "NoCollision")
  (`SceneComponent.SetVisibility` _mesh_base false false)
  (`self.K2_DestroyActor`))

(event `self.ReceiveBeginPlay`
  ;[1 1 1] Begin
  (bind _asbp_first_person_character (cast `/Game/FirstPerson/Blueprints/BP_FirstPersonCharacter` (`GameplayStatics.GetPlayerCharacter` 0) :!label _label)
    (:`then`
      (set `self.Character` _asbp_first_person_character))
    (:`CastFailed`
      (`KismetSystemLibrary.Delay` 0.2)
      (goto _label))))

(event `Key 2`
  ;[0 1 0.9272] Behaviour Key
  (set `/Game/FirstPerson/Blueprints/BP_FirstPersonCharacter.Key 2` (+ (`/Game/FirstPerson/Blueprints/BP_FirstPersonCharacter.Key 2` (`self.Character`)) (`self.Key +1`)) (`self.Character`)))

(event `CustomEvent`
  ;[0 1 0.9272] Behaviour Key
  (if true
    (`KismetSystemLibrary.LogString` "Tiene la llave")))

(event `self.ColliderBase.OnComponentBeginOverlap`
  (params (OverlappedComponent :type "PrimitiveComponent Object Reference") (OtherActor :type "Actor Object Reference") (OtherComp :type "PrimitiveComponent Object Reference") (OtherBodyIndex :type Integer) (bFromSweep :type Boolean) (SweepResult :type "HitResult Structure (by ref)"))
  ;[0.8253 0.5709 1] Collision
  (if (== OtherActor (`GameplayStatics.GetPlayerCharacter` 0))
    (`|ExecutionSequence`
      (:`then_0`
        (`self.PickUp`))
      (:`then_1`
        (`self.Key 2`))
      (:`then_2`
        (`KismetSystemLibrary.PrintString` (`KismetStringLibrary.Conv_DoubleToString` (`/Game/FirstPerson/Blueprints/BP_FirstPersonCharacter.Key 2` (`self.Character`)))))
      (:`then_3`
        (`self.K2_DestroyActor`)))))

(fn `UserConstructionScript`
  (bind _mesh_base (`self.Mesh Base`))
  (`StaticMeshComponent.SetStaticMesh` _mesh_base (`self.Mesh Change`))
  (`PrimitiveComponent.SetMaterial` _mesh_base 0 (`self.Material_1`)))