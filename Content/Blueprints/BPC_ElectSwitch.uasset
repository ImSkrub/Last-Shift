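; Electricity switch actor that turns the power on when interacted with.
; OnInteract plays a timeline that rolls the Switch component up to -90 degrees.
; A DoOnce on the timeline's update plays the lights-on sound on the first update, then sets ElectricityIsOn after a short delay.
; It has no logic for switching the power back off.
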(event `/Game/FirstPerson/Blueprints/BPI_Interact.OnInteract`
  (params (InteractingPlayer :type "/Game/FirstPerson/Blueprints/BP_FirstPersonCharacter Object Reference"))
  (bind _switch (`self.Switch`))
  (bind (_relativerotation_roll _relativerotation_pitch _relativerotation_yaw) (`KismetMathLibrary.BreakRotator` (`SceneComponent.RelativeRotation` _switch)))
  ;[1 1 1] Interact with Switch
  (bind (_direction _alphatrigger) (`Timeline|TriggerTL`)
    (:`Update`
      (`SceneComponent.K2_SetRelativeRotation` _switch (`KismetMathLibrary.MakeRotator` (* _alphatrigger -90.0) _relativerotation_pitch _relativerotation_yaw) false false)
      (`/Engine/EditorBlueprintResources/StandardMacros.DoOnce` false
        (:`Completed`
          (`GameplayStatics.PlaySoundAtLocation` "/Game/Audio/LightsOn.LightsOn" (`self.K2_GetActorLocation`) (struct) 1.0 1.0 0.0 null null null null)
          (`KismetSystemLibrary.Delay` 2.0)
          (set `self.ElectricityIsOn` true))))))

(fn `UserConstructionScript`
  (`parent.UserConstructionScript`))