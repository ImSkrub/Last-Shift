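; Blue door actor that swings open when its overlap component is triggered while the referenced character holds Key2.
; The overlap passes a CanOpen check and a DoOnce, then plays a timeline that lerps the door mesh's relative rotation from Closed to Open.
; On finish, a FlipFlop first clears CanOpen and resets the DoOnce, blocking further openings; nothing here closes the door.
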(event `self.Overlap.OnComponentBeginOverlap`
  (params (OverlappedComponent :type "PrimitiveComponent Object Reference") (OtherActor :type "Actor Object Reference") (OtherComp :type "PrimitiveComponent Object Reference") (OtherBodyIndex :type Integer) (bFromSweep :type Boolean) (SweepResult :type "HitResult Structure (by ref)"))
  ;[1 0.944 0.7197] Open Door
  (if (`/Game/FirstPerson/Blueprints/BP_FirstPersonCharacter.Key 2` (`self.CharacterRef`))
    (if (`self.canOpen`)
      (`/Engine/EditorBlueprintResources/StandardMacros.DoOnce` false :!label _label
        (:`Completed`
          (bind (_direction _speed) (`Timeline|Timeline_0`)
            (:`Update`
              (`SceneComponent.K2_SetRelativeRotation` (`self.SM_Door`) (`KismetMathLibrary.RLerp` (`self.Closed`) (`self.Open`) _speed) false false))
            (:`Finished`
              (`/Engine/EditorBlueprintResources/StandardMacros.FlipFlop`
                (:`A`
                  (set `self.canOpen` false)
                  (goto _label :!via `Reset`))
                (:`B`
                  (set `self.canOpen` true))))))))))

(fn `UserConstructionScript`
  (`parent.UserConstructionScript`))