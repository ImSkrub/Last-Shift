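; BP_Puerta is a door that swings open or closed on Box overlap once the first-person character holds at least one Moneditas.
; A Timeline lerps SMDoor's rotation, with DoOnce and FlipFlop tracking IsClosed to choose play or reverse.
; The construction script assigns the two door materials.
; Two key-based copies of the door logic are unconnected, so CollectItem's LLAVE counter does not affect the live door.
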(event `CollectItem`
  (params (OverlappedComponent :type "PrimitiveComponent Object Reference") (OtherActor :type "Actor Object Reference") (OtherComp :type "PrimitiveComponent Object Reference") (OtherBodyIndex :type Integer) (bFromSweep :type Boolean) (SweepResult :type "HitResult Structure (by ref)"))
  (bind _result (`/Engine/EditorBlueprintResources/StandardMacros.IncrementInt` (`self.LLAVE`))
    (:`  `
      (if true
        (set `self.LLAVE` _result)))))

(event `self.Box.OnComponentBeginOverlap`
  (params (OverlappedComponent :type "PrimitiveComponent Object Reference") (OtherActor :type "Actor Object Reference") (OtherComp :type "PrimitiveComponent Object Reference") (OtherBodyIndex :type Integer) (bFromSweep :type Boolean) (SweepResult :type "HitResult Structure (by ref)"))
  ;[1 1 1] Abrir Y Cerrar Puerta
  (if (>= (`/Game/FirstPerson/Blueprints/BP_FirstPersonCharacter.Moneditas` (`self.Padree`)) 1)
    (if (`self.IsClosed`)
      (`/Engine/EditorBlueprintResources/StandardMacros.DoOnce` false :!label _label
        (:`Completed`
          (bind (_direction _speed) (`Timeline|Timeline_0` :!via `PlayFromStart` :!label _label_2)
            (:`Update`
              (`SceneComponent.K2_SetRelativeRotation` (`self.SM_Door`) (`KismetMathLibrary.RLerp` (`self.Cerrada`) (`self.Abierta`) _speed) false false))
            (:`Finished`
              (`/Engine/EditorBlueprintResources/StandardMacros.FlipFlop`
                (:`A`
                  (set `self.IsClosed` false)
                  (goto _label :!via `Reset`))
                (:`B`
                  (set `self.IsClosed` true)))))))
      (else
        (goto _label_2 :!via `ReverseFromEnd`)))))

(event `self.ReceiveBeginPlay`
  (bind _asbp_first_person_character (cast `/Game/FirstPerson/Blueprints/BP_FirstPersonCharacter` (`GameplayStatics.GetPlayerCharacter` 0)))
  (set `self.Padree` _asbp_first_person_character))

(fn `UserConstructionScript`
  (bind _sm_door (`self.SM_Door`))
  (`PrimitiveComponent.SetMaterial` _sm_door 0 (`self.MaterialCuerpo`))
  (`PrimitiveComponent.SetMaterial` _sm_door 1 (`self.MaterialTransparente`)))