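; Door Blueprint that swings open when its overlap box is triggered while the first-person character holds at least one Key3.
; BeginPlay caches the character, retrying after a short delay until the cast succeeds.
; A timeline lerps the door's rotation from Closed to Open, gated by CanOpen and a DoOnce; its first finish clears CanOpen, blocking further triggers.
; The construction script applies configurable door and glass materials.
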(event `self.ReceiveBeginPlay`
  ;[1 1 1] Begin
  (bind _asbp_first_person_character (cast `/Game/FirstPerson/Blueprints/BP_FirstPersonCharacter` (`GameplayStatics.GetPlayerCharacter` 0) :!label _label)
    (:`then`
      (set `self.CharacterRef` _asbp_first_person_character))
    (:`CastFailed`
      (`KismetSystemLibrary.Delay` 0.2)
      (goto _label))))

(event `self.overlapBox.OnComponentBeginOverlap`
  (params (OverlappedComponent :type "PrimitiveComponent Object Reference") (OtherActor :type "Actor Object Reference") (OtherComp :type "PrimitiveComponent Object Reference") (OtherBodyIndex :type Integer) (bFromSweep :type Boolean) (SweepResult :type "HitResult Structure (by ref)"))
  ;[1 0.6332 0.3338] Open/Close Door
  (if (>= (`/Game/FirstPerson/Blueprints/BP_FirstPersonCharacter.Key 3` (`self.CharacterRef`)) 1.0)
    (if (`self.canOpen`)
      (`/Engine/EditorBlueprintResources/StandardMacros.DoOnce` false :!label _label_2
        (:`Completed`
          (bind (_direction _speed) (`Timeline|DoorTimeline` :!via `PlayFromStart`)
            (:`Update`
              (`SceneComponent.K2_SetRelativeRotation` (`self.SM_Door`) (`KismetMathLibrary.RLerp` (`self.Closed`) (`self.Open`) _speed) false false))
            (:`Finished`
              (`/Engine/EditorBlueprintResources/StandardMacros.FlipFlop`
                (:`A`
                  (set `self.canOpen` false)
                  (goto _label_2 :!via `Reset`))
                (:`B`
                  (set `self.canOpen` true))))))))))

(fn `UserConstructionScript`
  (bind _sm_door (`self.SM_Door`))
  (`PrimitiveComponent.SetMaterial` _sm_door 0 (`self.Door Material`))
  (`PrimitiveComponent.SetMaterial` _sm_door 1 (`self.Glass Material`)))