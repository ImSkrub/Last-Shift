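; BP_ElecTrigger is an interactable electrical switch that turns a lights-on flag on when used.
; OnInteract plays the SwitchTL timeline, whose alpha rolls the Trigger component up to 90 degrees while keeping its pitch and yaw.
; Timeline updates also set LightsAreOn, and a DoOnce plays the LightsOn sound at the actor's location a single time.
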(event `/Game/FirstPerson/Blueprints/BPI_Interact.OnInteract`
  (params (InteractingPlayer :type "/Game/FirstPerson/Blueprints/BP_FirstPersonCharacter Object Reference"))
  (bind _trigger (`self.Trigger`))
  (bind (_relativerotation_roll _relativerotation_pitch _relativerotation_yaw) (`KismetMathLibrary.BreakRotator` (`SceneComponent.RelativeRotation` _trigger)))
  (bind (_direction _alphaswitch) (`Timeline|SwitchTL`)
    (:`Update`
      (`SceneComponent.K2_SetRelativeRotation` _trigger (`KismetMathLibrary.MakeRotator` (* _alphaswitch 90.0) _relativerotation_pitch _relativerotation_yaw) false false)
      (`|ExecutionSequence`
        (:`then_0`
          (set `self.LightsAreOn` true))
        (:`then_1`
          (`/Engine/EditorBlueprintResources/StandardMacros.DoOnce` false
            (:`Completed`
              (`GameplayStatics.PlaySoundAtLocation` "/Game/Audio/LightsOn.LightsOn" (`self.K2_GetActorLocation`) (struct) 1.0 1.0 0.0 null null null null))))))))

(fn `UserConstructionScript`
  (`parent.UserConstructionScript`))