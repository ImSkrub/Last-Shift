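; BP_Switchboard is an interactable switchboard actor with animated open, close and switch states.
; A box overlap plays the open animation through an unreset DoOnce followed by a player check; the player leaving plays the close animation.
; OnInteract plays the switch animation and activates an effect set visible in scene capture only.
; After a delay, it either restarts the effect in a loop or destroys the actor, depending on IsLoop.
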(event `self.ReceiveBeginPlay`
  (set `self.CurrentTime` 0.0))

(event `self.Box.OnComponentBeginOverlap`
  (params (OverlappedComponent :type "PrimitiveComponent Object Reference") (OtherActor :type "Actor Object Reference") (OtherComp :type "PrimitiveComponent Object Reference") (OtherBodyIndex :type Integer) (bFromSweep :type Boolean) (SweepResult :type "HitResult Structure (by ref)"))
  (`/Engine/EditorBlueprintResources/StandardMacros.DoOnce` false
    (:`Completed`
      (if (== OtherActor (`GameplayStatics.GetPlayerCharacter` 0))
        (`SkeletalMeshComponent.PlayAnimation` (`self.switchboard1`) "/Game/Fab/Switchboard/switchboard_AnimOpen.switchboard_AnimOpen" false)))))

(event `self.Box.OnComponentEndOverlap`
  (params (OverlappedComponent :type "PrimitiveComponent Object Reference") (OtherActor :type "Actor Object Reference") (OtherComp :type "PrimitiveComponent Object Reference") (OtherBodyIndex :type Integer))
  (if (== (`GameplayStatics.GetPlayerCharacter` 0) OtherActor)
    (`SkeletalMeshComponent.PlayAnimation` (`self.switchboard1`) "/Game/Fab/Switchboard/switchboard_AnimClose.switchboard_AnimClose" false)))

(event `/Game/FirstPerson/Blueprints/BPI_Interact.OnInteract`
  (params (InteractingPlayer :type "/Game/FirstPerson/Blueprints/BP_FirstPersonCharacter Object Reference"))
  (bind _effect (`self.Effect`))
  (`KismetSystemLibrary.PrintString` "Interacted")
  (`SkeletalMeshComponent.PlayAnimation` (`self.switchboard1`) "/Game/Fab/Switchboard/Switch.Switch" false)
  (`PrimitiveComponent.SetVisibleInSceneCaptureOnly` (`self.Effect`) true)
  (`ActorComponent.Activate` _effect false :!label _label)
  (`KismetSystemLibrary.Delay` (`self.VFX interval`))
  (if (`self.IsLoop`)
    (`ActorComponent.Deactivate` _effect)
    (goto _label)
    (else
      (`self.K2_DestroyActor`))))

(fn `UserConstructionScript`)