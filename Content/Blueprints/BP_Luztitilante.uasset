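; Flickering ceiling lamp actor with a configurable mesh, rect light and activation sphere.
; Construction script applies the mesh, scale, light color, intensity, attenuation and sphere radius.
; Tick runs Flickering: while Triggered, a self-resetting DoOnce sets a fixed intensity and toggles visibility after nested-random delays; otherwise intensity drops to zero.
; Nothing here sets Triggered or handles sphere overlaps.
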(event `self.ReceiveTick`
  (params (DeltaSeconds :type "Float (single-precision)"))
  (`self.Flickering`))

(event `Flickering`
  (bind _rectlight (`self.RectLight`))
  (if (`self.Triggered`)
    (`/Engine/EditorBlueprintResources/StandardMacros.DoOnce` false :!label _label
      (:`Completed`
        (`LightComponent.SetIntensity` _rectlight 50.0)
        (`KismetSystemLibrary.RetriggerableDelay` (`KismetMathLibrary.RandomFloatInRange` (`KismetMathLibrary.RandomFloatInRange` 0.001 0.75) (`KismetMathLibrary.RandomFloatInRange` 0.02 0.75)))
        (`SceneComponent.ToggleVisibility` (`self.RectLight`) false)
        (goto _label :!via `Reset`)))
    (else
      (`LightComponent.SetIntensity` _rectlight 0.0))))

(fn `UserConstructionScript`
  (bind _sm_lamp_ceiling (`self.SM_Lamp_Ceiling`))
  (`|ExecutionSequence`
    (:`then_0`
      ;[1 1 1] Set static mesh
      (`StaticMeshComponent.SetStaticMesh` (`self.SM_Lamp_Ceiling`) (`self.Light mesh`))
      ;[1 1 1] Set Transform dynamically
      (`SceneComponent.K2_SetWorldTransform` _sm_lamp_ceiling (`KismetMathLibrary.MakeTransform` (`SceneComponent.K2_GetComponentLocation` _sm_lamp_ceiling) (`SceneComponent.K2_GetComponentRotation` _sm_lamp_ceiling) (`self.Light Mesh Scale`)) false false))
    (:`then_1`
      ;[1 1 1] Light values
      (`LightComponent.SetIntensity` (`self.RectLight`) (`self.Light Intensity`))
      (`LightComponent.SetLightColor` (`self.RectLight`) (`self.New Light Color`) true)
      (`LocalLightComponent.SetAttenuationRadius` (`self.RectLight`) (`self.New AttenuationRadius`)))
    (:`then_2`
      (`SphereComponent.SetSphereRadius` (`self.ActivationRadius`) (`self.SphereRadius`) true))))