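; Interactable key pickup that, depending on its flags, opens up a vent or unlocks a door when collected.
; With DestornilladorVioleta set it calls IsOpen on an assigned vent; with Keycard set, on the vent nearest the character.
; Otherwise it sets CanOpen on the nearest door.
; Interaction then shows the animated WBP_Tarjeta card widget and destroys the actor.
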(event `PickUp`
  ;[1 1 1] Pick up
  (if (`self.destornilladorVioleta`)
    (bind _asbp_vent (cast `/Game/Blueprints/BP_Vent` (`self.destornilladorVentRef`)))
    (`/Game/Blueprints/BP_Vent.IsOpen` _asbp_vent)
    (elif (`self.Keycard?`)
      (bind _outactors (`GameplayStatics.GetAllActorsOfClass` "/Game/Blueprints/BP_Vent.BP_Vent_C"))
      (bind _output_get (set `self.NearVentRef` (`.ReturnValue` (`GameplayStatics.FindNearestActor` (`self.K2_GetActorLocation` (`self.CharacterRef`)) _outactors))))
      (bind _asbp_vent_2 (cast `/Game/Blueprints/BP_Vent` _output_get))
      (`/Game/Blueprints/BP_Vent.IsOpen` _asbp_vent_2)
      (else
        (bind _outactors_2 (`GameplayStatics.GetAllActorsOfClass` "/Game/FirstPerson/Blueprints/BP_Door.BP_Door_C"))
        (bind _output_get_2 (set `self.NearDoor Ref` (`.ReturnValue` (`GameplayStatics.FindNearestActor` (`self.K2_GetActorLocation` (`self.CharacterRef`)) _outactors_2))))
        (bind _asbp_door (cast `/Game/FirstPerson/Blueprints/BP_Door` _output_get_2))
        (set `/Game/FirstPerson/Blueprints/BP_Door.CanOpen?` true _asbp_door)))))

(event `/Game/FirstPerson/Blueprints/BPI_Interact.OnInteract`
  (params (InteractingPlayer :type "/Game/FirstPerson/Blueprints/BP_FirstPersonCharacter Object Reference"))
  (`|ExecutionSequence`
    (:`then_0`
      (`self.PickUp`))
    (:`then_2`
      (bind _returnvalue (`|CreateWidget` "/Game/Widgets/WBP_Tarjeta.WBP_Tarjeta_C"))
      (`UserWidget.AddToViewport` _returnvalue 0)
      (`/Game/Widgets/WBP_Tarjeta.Play Tarjeta Animacion` _returnvalue))
    (:`then_3`
      (`self.K2_DestroyActor`))))

(fn `UserConstructionScript`
  (`parent.UserConstructionScript`))