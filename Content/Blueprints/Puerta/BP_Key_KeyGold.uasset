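; Gold key pickup that flags the player character as holding key 3 and then removes itself.
; Overlap of ColliderBase by player character 0 runs PickUp, sets Key3 on the Character reference, prints the flag and destroys the actor.
; A separate LogKey event logs a Spanish "has the key" message when that flag is set, but nothing in this graph calls it.
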(event `Log Key`
  ;[0 1 0.9272] Behaviour Key
  (if (`/Game/FirstPerson/Blueprints/BP_FirstPersonCharacter.Key 3` (`self.Character`))
    (`KismetSystemLibrary.LogString` "Tiene la llave")))

(event `Key3`
  ;[0 1 0.9272] Behaviour Key
  (set `/Game/FirstPerson/Blueprints/BP_FirstPersonCharacter.Key 3` true (`self.Character`)))

(event `self.ColliderBase.OnComponentBeginOverlap`
  (params (OverlappedComponent :type "PrimitiveComponent Object Reference") (OtherActor :type "Actor Object Reference") (OtherComp :type "PrimitiveComponent Object Reference") (OtherBodyIndex :type Integer) (bFromSweep :type Boolean) (SweepResult :type "HitResult Structure (by ref)"))
  ;[1 1 1] Colision
  (if (== OtherActor (`GameplayStatics.GetPlayerCharacter` 0))
    (`|ExecutionSequence`
      (:`then_0`
        (`self.PickUp`))
      (:`then_1`
        (`self.Key3`))
      (:`then_2`
        (`KismetSystemLibrary.PrintString` (`KismetStringLibrary.Conv_BoolToString` (`/Game/FirstPerson/Blueprints/BP_FirstPersonCharacter.Key 3` (`self.Character`)))))
      (:`then_3`
        (`self.K2_DestroyActor`)))))

(fn `UserConstructionScript`
  (`parent.UserConstructionScript`))