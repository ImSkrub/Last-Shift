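; BP_SwitchPanel is a switchboard actor that animates the first time the player character enters its box trigger.
; The overlap passes a DoOnce, starts the non-looping switchboard animation, then immediately sets the freeze-pose animation through an always-true branch, with no delay between them.
; A separate OnInteract event clears IsFrozen and zeroes CurrentTime when frozen, though nothing in these graphs sets IsFrozen true or reads CurrentTime.
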(event `self.Box.OnComponentBeginOverlap`
  (params (OverlappedComponent :type "PrimitiveComponent Object Reference") (OtherActor :type "Actor Object Reference") (OtherComp :type "PrimitiveComponent Object Reference") (OtherBodyIndex :type Integer) (bFromSweep :type Boolean) (SweepResult :type "HitResult Structure (by ref)"))
  (if (== OtherActor (`GameplayStatics.GetPlayerCharacter` 0))
    (`/Engine/EditorBlueprintResources/StandardMacros.DoOnce` false
      (:`Completed`
        (`SkeletalMeshComponent.PlayAnimation` (`self.switchboard1`) "/Game/Fab/Switchboard/switchboard_Anim.switchboard_Anim" false)
        (if true
          (`SkeletalMeshComponent.SetAnimation` (`self.switchboard1`) "/Game/Fab/Switchboard/FreezePose_Switchboard.FreezePose_Switchboard"))))))

(event `/Game/FirstPerson/Blueprints/BPI_Interact.OnInteract`
  (params (InteractingPlayer :type "/Game/FirstPerson/Blueprints/BP_FirstPersonCharacter Object Reference"))
  (if (`self.bIsFrozen`)
    (set `self.bIsFrozen` false)
    (set `self.currentTime` 0.0)))

(fn `UserConstructionScript`)