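; BP_PickUp is a coin pickup that adds its Moneditas value to the first-person character when the player walks into it.
; BeginPlay caches the character as Padree, and the box overlap calls PickUp to hide and destroy the actor, then DaMoneda to add coins and prints the total.
; The construction script applies the MeshChange mesh to MeshBase.
; A BP_Puerta CollectItem call is left unconnected.
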(event `PickUp`
  (bind _mesh_base (`self.Mesh Base`))
  (`PrimitiveComponent.SetCollisionEnabled` _mesh_base "NoCollision")
  (`SceneComponent.SetVisibility` _mesh_base false false)
  (`self.K2_DestroyActor`))

(event `self.ReceiveBeginPlay`
  (bind _asbp_first_person_character (cast `/Game/FirstPerson/Blueprints/BP_FirstPersonCharacter` (`GameplayStatics.GetPlayerCharacter` 0)))
  (set `self.padree` _asbp_first_person_character))

(event `Da Moneda`
  (set `/Game/FirstPerson/Blueprints/BP_FirstPersonCharacter.Moneditas` (+ (`/Game/FirstPerson/Blueprints/BP_FirstPersonCharacter.Moneditas` (`self.padree`)) (`self.Moneditas`)) (`self.padree`)))

(event `self.Box.OnComponentBeginOverlap`
  (params (OverlappedComponent :type "PrimitiveComponent Object Reference") (OtherActor :type "Actor Object Reference") (OtherComp :type "PrimitiveComponent Object Reference") (OtherBodyIndex :type Integer) (bFromSweep :type Boolean) (SweepResult :type "HitResult Structure (by ref)"))
  (if (== OtherActor (`GameplayStatics.GetPlayerCharacter` 0))
    (`self.PickUp`)
    (`self.Da Moneda`)
    (`KismetSystemLibrary.PrintString` (`KismetStringLibrary.Conv_DoubleToString` (`/Game/FirstPerson/Blueprints/BP_FirstPersonCharacter.Moneditas` (`self.padree`))))
    (`self.K2_DestroyActor`)))

(fn `UserConstructionScript`
  (`StaticMeshComponent.SetStaticMesh` (`self.Mesh Base`) (`self.Mesh Change`)))