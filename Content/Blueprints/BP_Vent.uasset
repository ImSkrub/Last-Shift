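; Interactable vent that, once flagged by its IsOpen event, unscrews and swings open on interaction.
; A timeline spins and slides the screw, then after a delay a second timeline rotates the vent mesh as the screw is destroyed.
; Nested outer and inner overlap spheres swap two prompt icons as the player approaches.
; Outer end-overlap compares the player to the overlapped component, so that icon's hide check does not match.
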(event `IsOpen`
  (set `self.IsOpen?` true))

(event `/Game/FirstPerson/Blueprints/BPI_Interact.OnInteract`
  (params (InteractingPlayer :type "/Game/FirstPerson/Blueprints/BP_FirstPersonCharacter Object Reference"))
  (bind _screw (`self.Screw`))
  (if (`self.IsOpen?`)
    (`|ExecutionSequence`
      (:`then_0`
        (bind (_direction _newtrack_0 _location) (`Timeline|ScrewTimeline`)
          (:`Update`
            (`SceneComponent.K2_SetRelativeRotation` _screw (`KismetMathLibrary.MakeRotator` 90.0 (* _newtrack_0 720.0)) false false)
            (`SceneComponent.K2_SetRelativeLocation` _screw (`KismetMathLibrary.MakeVector` 67.0 (* _location 20.0)) false false))))
      (:`then_1`
        (`KismetSystemLibrary.Delay` 2.0)
        (`|ExecutionSequence`
          (:`then_0`
            (bind (_direction_2 _ventalpha) (`Timeline|Vent Timeline`)
              (:`Update`
                (`SceneComponent.K2_SetRelativeRotation` (`self.VentMesh`) (`KismetMathLibrary.MakeRotator` (* _ventalpha -90.0)) false false))))
          (:`then_1`
            (`ActorComponent.K2_DestroyComponent` (`self.Screw`))))))))

(event `self.OuterSphereColision.OnComponentBeginOverlap`
  (params (OverlappedComponent :type "PrimitiveComponent Object Reference") (OtherActor :type "Actor Object Reference") (OtherComp :type "PrimitiveComponent Object Reference") (OtherBodyIndex :type Integer) (bFromSweep :type Boolean) (SweepResult :type "HitResult Structure (by ref)"))
  (if (== OtherActor (`GameplayStatics.GetPlayerCharacter` 0))
    (`SceneComponent.SetVisibility` (`self.OuterIcon`) true false)))

(event `self.InnerSphereColision.OnComponentBeginOverlap`
  (params (OverlappedComponent :type "PrimitiveComponent Object Reference") (OtherActor :type "Actor Object Reference") (OtherComp :type "PrimitiveComponent Object Reference") (OtherBodyIndex :type Integer) (bFromSweep :type Boolean) (SweepResult :type "HitResult Structure (by ref)"))
  (if (== OtherActor (`GameplayStatics.GetPlayerCharacter` 0))
    (`SceneComponent.SetVisibility` (`self.Inner Icon`) true false)
    (`SceneComponent.SetVisibility` (`self.OuterIcon`) false false)))

(event `self.InnerSphereColision.OnComponentEndOverlap`
  (params (OverlappedComponent :type "PrimitiveComponent Object Reference") (OtherActor :type "Actor Object Reference") (OtherComp :type "PrimitiveComponent Object Reference") (OtherBodyIndex :type Integer))
  (if (== (`GameplayStatics.GetPlayerCharacter` 0) OtherActor)
    (`SceneComponent.SetVisibility` (`self.Inner Icon`) false false)
    (`SceneComponent.SetVisibility` (`self.OuterIcon`) true false)))

(event `self.OuterSphereColision.OnComponentEndOverlap`
  (params (OverlappedComponent :type "PrimitiveComponent Object Reference") (OtherActor :type "Actor Object Reference") (OtherComp :type "PrimitiveComponent Object Reference") (OtherBodyIndex :type Integer))
  (if (== (`GameplayStatics.GetPlayerCharacter` 0) OverlappedComponent)
    (`SceneComponent.SetVisibility` (`self.OuterIcon`) false false)))

(fn `UserConstructionScript`)