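; BP_KeycardPanel is a two-sided door control panel that unlocks or locks the door closest to it.
; On BeginPlay it gathers all BP_Door actors and caches the nearest one, so the link comes from placement.
; On interact it reads ElectricityOn, swaps both panels to the open or closed lock material and sets the door's CanOpen to match.
; Despite the name, the graph checks only power, with no keycard test.
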(event `self.ReceiveBeginPlay`
  (bind _outactors (`GameplayStatics.GetAllActorsOfClass` "/Game/FirstPerson/Blueprints/BP_Door.BP_Door_C"))
  (bind _output_get (set `self.NearDoorRef` (`.ReturnValue` (`GameplayStatics.FindNearestActor` (`self.K2_GetActorLocation`) _outactors))))
  (bind _asbp_door (cast `/Game/FirstPerson/Blueprints/BP_Door` _output_get))
  (set `self.As BP Door` _asbp_door))

(event `/Game/FirstPerson/Blueprints/BPI_Interact.OnInteract`
  (params (InteractingPlayer :type "/Game/FirstPerson/Blueprints/BP_FirstPersonCharacter Object Reference"))
  (bind _controlpanel (`self.ControlPanel`))
  (bind _controlpanelotherside (`self.ControlPanelOtherSide`))
  (if (`self.Electricity On`)
    (`PrimitiveComponent.SetMaterial` _controlpanel 1 (`self.Open Lock`))
    (`PrimitiveComponent.SetMaterial` _controlpanelotherside 1 (`self.Open Lock`))
    (set `/Game/FirstPerson/Blueprints/BP_Door.CanOpen?` true (`self.As BP Door`))
    (else
      (`PrimitiveComponent.SetMaterial` _controlpanel 1 (`self.Closed lock`))
      (`PrimitiveComponent.SetMaterial` _controlpanelotherside 1 (`self.Closed lock`))
      (set `/Game/FirstPerson/Blueprints/BP_Door.CanOpen?` false (`self.As BP Door`)))))

(fn `UserConstructionScript`)