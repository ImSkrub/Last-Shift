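; BP_Statue is a collectible statue that hops around the play area for the player to catch.
; InitStatue teleports it to a random floor position and re-arms itself on a timer that shortens as the GM_CachitoPremium level rises.
; On player overlap before game over, it notifies the game mode, plays dust and collapse sound, calls CallHola, destroys itself and spawns a replacement, which relocates on BeginPlay.
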(event `self.ReceiveBeginPlay`
  (bind _asgm_cachito_premium (cast `/Game/BP/GM_CachitoPremium` (`GameplayStatics.GetGameMode`)))
  (set `self.GM_Cachito` _asgm_cachito_premium)
  (`self.InitStatue`))

(event `self.ReceiveActorBeginOverlap`
  (params (OtherActor :type "Actor Object Reference"))
  (bind _returnvalue (`self.K2_GetActorLocation`))
  (if (and (== OtherActor (`GameplayStatics.GetPlayerCharacter` 0)) (not (`/Game/BP/GM_CachitoPremium.GameOver` (`self.GM_Cachito`))))
    (`/Game/BP/GM_CachitoPremium.StatueCollected` (`self.GM_Cachito`))
    (`GameplayStatics.SpawnEmitterAtLocation` "/Game/StarterContent/Particles/P_Ambient_Dust.P_Ambient_Dust" _returnvalue)
    (`GameplayStatics.SpawnSoundAtLocation` "/Game/StarterContent/Audio/Collapse01.Collapse01" _returnvalue (struct) 1.0 1.0 0.0 null null)
    (`self.Hola`)
    (`self.K2_DestroyActor`)
    (`|SpawnActorFromClass` "BP_Statue_C" (`self.GetTransform`) "Undefined" "MultiplyWithRoot" null null)))

(fn `InitStatue`
  (`self.K2_TeleportTo` (`KismetMathLibrary.MakeVector` (`KismetMathLibrary.RandomFloatInRange` 300.0 1800.0) (`KismetMathLibrary.RandomFloatInRange` 250.0 1650.0)))
  (`KismetSystemLibrary.K2_SetTimer` null "InitStatue" (`KismetMathLibrary.Conv_IntToDouble` (- 6 (`/Game/BP/GM_CachitoPremium.Level` (`self.GM_Cachito`))))))

(fn `UserConstructionScript`)