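; BP_GUIDE_HUD is a HUD Blueprint that draws the game's score, time and level, plus a Game Over message.
; On BeginPlay it casts the game mode to GM_CachitoPremium and caches the reference.
; Each DrawHUD reads that reference and draws colored text at fixed screen coordinates along the top.
; When the GameOver flag is set it adds large red text mid-screen; the second of those draw calls has no text assigned.
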(event `self.ReceiveBeginPlay`
  (bind _asgm_cachito_premium (cast `/Game/BP/GM_CachitoPremium` (`GameplayStatics.GetGameMode`)))
  (set `self.GM_Ref` _asgm_cachito_premium))

(event `self.ReceiveDrawHUD`
  (params (SizeX :type Integer) (SizeY :type Integer))
  (`self.DrawText` (`KismetStringLibrary.BuildString_Int` "Score: " "" (`/Game/BP/GM_CachitoPremium.Score` (`self.GM_Ref`))) (struct :`R` 0.024507 :`G` 1.0 :`A` 1.0) 10.0 10.0 null 2.0)
  (`self.DrawText` (`KismetStringLibrary.BuildString_Int` "" "" (`/Game/BP/GM_CachitoPremium.Time` (`self.GM_Ref`))) (struct :`R` 1.0 :`G` 0.153938 :`B` 0.213676 :`A` 1.0) 1000.0 10.0 null 2.0)
  (`self.DrawText` (`KismetStringLibrary.BuildString_Int` "" "" (`/Game/BP/GM_CachitoPremium.Level` (`self.GM_Ref`))) (struct :`G` 0.626192 :`B` 1.0 :`A` 1.0) 1800.0 10.0 null 2.0)
  (if (`/Game/BP/GM_CachitoPremium.GameOver` (`self.GM_Ref`))
    (`self.DrawText` "Game Over" (struct :`R` 1.0 :`G` 0.021217 :`A` 1.0) 800.0 490.0 null 5.0)
    (`self.DrawText` "" (struct :`R` 1.0 :`G` 0.10353 :`A` 1.0) 800.0 520.0 null 5.0)))

(fn `UserConstructionScript`)