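; Game mode for a timed statue-collecting game that tracks score, level, remaining time and game-over state.
; StartGame resets that state on BeginPlay or RestartGame and starts a looping one-second Clock timer that counts down and ends the game at zero.
; StatueCollected awards points scaled by level, and every fifth statue adds bonus time and raises the level up to a cap.
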(event `self.ReceiveBeginPlay`
  (`self.StartGame`))

(event `Restart Game`
  (`self.StartGame`))

(event `Clock`
  (bind _output_get (set `self.Time` (- (`self.Time`) 1)))
  (if (== _output_get 0)
    (set `self.GameOver` true)
    (`KismetSystemLibrary.K2_ClearTimer` null "Clock")))

(fn `StatueCollected`
  (set `self.Score` (+ (`self.Score`) (* (`self.Level`) 10)))
  (bind _output_get (set `self.StatueCount` (+ (`self.StatueCount`) 1)))
  (if (== (mod _output_get 5) 0)
    (set `self.Time` (+ (`self.Time`) 15))
    (set `self.Level` (`KismetMathLibrary.Min` (+ (`self.Level`) 1) 5))))

(fn `UserConstructionScript`)